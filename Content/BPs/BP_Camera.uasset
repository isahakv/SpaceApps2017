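; BP_Camera is an orbit camera that attaches to the first BP_Asteroid found, snapping to its transform and enabling player input.
; Horizontal input yaws the spring arm, while vertical input rolls the whole actor in world space.
; Zoom input changes arm length with a minimum distance but no maximum.
; Pressing Z plays a timeline that eases the spring arm's relative rotation back to zero.
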(event `self.ReceiveBeginPlay`
  (set `SpringArmComponent.TargetArmLength` (`self.MinDistance`) (`self.SpringArm`)))

(event `InputAxis|Horizontal`
  (params (AxisValue :type "Float (single-precision)"))
  (`SceneComponent.K2_AddRelativeRotation` (`self.SpringArm`) (`KismetMathLibrary.MakeRotator` 0.0 0.0 (* AxisValue (`self.Speed`))) false false))

(event `InputAxis|Zoom`
  (params (AxisValue :type "Float (single-precision)"))
  (bind _springarm (`self.SpringArm`))
  (bind _returnvalue (+ (`SpringArmComponent.TargetArmLength` _springarm) (* AxisValue (`self.Speed`) 6.0)))
  (if (>= _returnvalue (`self.MinDistance`))
    (set `SpringArmComponent.TargetArmLength` _returnvalue _springarm)))

(event `InputAxis|Vertical`
  (params (AxisValue :type "Float (single-precision)"))
  (`self.K2_AddActorWorldRotation` (`KismetMathLibrary.MakeRotator` (* AxisValue (`self.Speed`)))))

(event `Key|Z`
  (params (Key :type "Key Structure" :default "AnyKey"))
  (:`Pressed`
    (bind (_direction _val) (`Timeline|Timeline_0`)
      (:`Update`
        (`SceneComponent.K2_SetRelativeRotation` (`self.SpringArm`) (`KismetMathLibrary.RLerp` (`SceneComponent.RelativeRotation` (`self.SpringArm`)) (struct) _val true) false false)))))

(fn `AttachToAsteroid`
  (bind _outactors (`GameplayStatics.GetAllActorsOfClass` "/Game/BPs/BP_Asteroid.BP_Asteroid_C"))
  (set `self.Darget` (`KismetArrayLibrary.Array_Get` _outactors))
  (`self.EnableInput` (`GameplayStatics.GetPlayerController` 0))
  (`self.K2_AttachToActor` (`self.Darget`) "None" "SnapToTarget" "SnapToTarget" "SnapToTarget"))

(fn `UserConstructionScript`)