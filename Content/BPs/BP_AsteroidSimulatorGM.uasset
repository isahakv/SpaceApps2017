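; Game mode for the asteroid simulator that sets up the scenario and controls the in-game pause menu.
; On BeginPlay it sets G, creates the HUD and menu widgets, caches the Earth actor, and spawns an asteroid.
; The asteroid's distance, direction, radius, mass and speed come from BP_GameInstance.
; The InGameMenu input toggles the menu, mouse cursor and game pause together.
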(event `self.ReceiveBeginPlay`
  (bind _output_get (set `self.G` 1.0))
  (`KismetSystemLibrary.PrintString` (`KismetStringLibrary.Conv_DoubleToString` _output_get) true true (struct :`G` 0.66 :`B` 1.0 :`A` 1.0) 10.0)
  (`self.EnableInput` (`GameplayStatics.GetPlayerController` 0))
  ;[1 1 1] UI
  (bind _returnvalue (`|CreateWidget` "/Game/UI/InGameMenu_WidgetBlueprint.InGameMenu_WidgetBlueprint_C"))
  (set `self.InGameMenuWidget` _returnvalue)
  (bind _returnvalue_2 (`|CreateWidget` "/Game/UI/HUD_WidgetBlueprint.HUD_WidgetBlueprint_C"))
  (bind _output_get_2 (set `self.HUDWidget` _returnvalue_2))
  (`UserWidget.AddToViewport` _output_get_2 0)
  ;[1 1 1] Get Earth
  (bind _outactors (`GameplayStatics.GetAllActorsOfClass` "/Game/BPs/BP_Earth.BP_Earth_C"))
  (set `self.Earth` (`KismetArrayLibrary.Array_Get` _outactors))
  (bind _asbp_game_instance (cast `/Game/BPs/BP_GameInstance` (`GameplayStatics.GetGameInstance`)))
  (bind _asteroiddirection (`/Game/BPs/BP_GameInstance.AsteroidDirection` _asbp_game_instance))
  (bind _returnvalue_3 (`|SpawnActorFromClass` "/Game/BPs/BP_Asteroid.BP_Asteroid_C" (`KismetMathLibrary.MakeTransform` (`KismetMathLibrary.MakeVector` (`/Game/BPs/BP_GameInstance.AsteroidDistanceFromEarth` _asbp_game_instance)) (`KismetMathLibrary.Conv_VectorToRotator` _asteroiddirection)) "AlwaysSpawn" "OverrideRootScale"))
  (bind _output_get_3 (set `self.Asteroid` _returnvalue_3))
  (`/Engine/EditorBlueprintResources/StandardMacros.IsValid` _output_get_3
    (:`Is Valid`
      (`/Game/BPs/BP_Asteroid.SetRadius` _output_get_3 (`/Game/BPs/BP_GameInstance.AsteroidRadiusInKm` _asbp_game_instance))
      (set `/Game/BPs/BP_Asteroid.Mass` (`/Game/BPs/BP_GameInstance.AsteroidMass` _asbp_game_instance) _output_get_3)
      (set `/Game/BPs/BP_Asteroid.velocity` (* _asteroiddirection (`/Game/BPs/BP_GameInstance.AsteroidSpeed` _asbp_game_instance)) _returnvalue_3))))

(event `InputAction|InGameMenu`
  (params (Key :type "Key Structure" :default "AnyKey"))
  (:`Pressed`
    (`self.ToggleInGameMenu` (not (`Widget.IsInViewport` (`self.InGameMenuWidget`))))))

(fn `ToggleInGameMenu`
  (params (enable :type Boolean))
  (bind _returnvalue (`GameplayStatics.GetPlayerController` 0))
  (bind _ingamemenuwidget (`self.InGameMenuWidget`))
  (bind _returnvalue_2 (`Widget.IsInViewport` _ingamemenuwidget))
  (if enable
    (if (not _returnvalue_2)
      (`UserWidget.AddToViewport` _ingamemenuwidget 0)
      (set `PlayerController.bShowMouseCursor` true _returnvalue)
      (`GameplayStatics.SetGamePaused` true))
    (elif _returnvalue_2
      (`Widget.RemoveFromParent` _ingamemenuwidget)
      (set `PlayerController.bShowMouseCursor` false _returnvalue)
      (`GameplayStatics.SetGamePaused` false))))

(fn `UserConstructionScript`)