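; Simulated asteroid that moves with swept offsets, explodes on overlapping BP_Earth and attaches the camera on spawn.
; Tick applies inverse-square gravity scaled by GameMode time multiplier (last Earth wins, BeginPlay zeroes G) and draws a debug-point trail.
; Hits branch on physical surface: Africa shows a radius-based death toll on the HUD, others only print.
; SetRadius resizes collision sphere and mesh together.
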(event `self.ReceiveBeginPlay`
  (bind _asbp_asteroid_simulator_gm (cast `/Game/BPs/BP_AsteroidSimulatorGM` (`GameplayStatics.GetGameMode`)))
  (set `self.GM` _asbp_asteroid_simulator_gm)
  (bind _output_get (set `self.G` 6.674e-12))
  (`KismetSystemLibrary.PrintString` (`KismetStringLibrary.Conv_DoubleToString` _output_get) true true (struct :`R` 1.0 :`G` 0.194582 :`B` 0.07485 :`A` 1.0))
  (bind _outactors (`GameplayStatics.GetAllActorsOfClass` "/Game/BPs/BP_Camera.BP_Camera_C"))
  (bind _asbp_camera (cast `/Game/BPs/BP_Camera` (`KismetArrayLibrary.Array_Get` _outactors)))
  (`/Game/BPs/BP_Camera.AttachToAsteroid` _asbp_camera))

(event `self.ReceiveTick`
  (params (DeltaSeconds :type "Float (single-precision)"))
  (bind _returnvalue (* DeltaSeconds (`/Game/BPs/BP_AsteroidSimulatorGM.timeMultiplier` (`self.GM`))))
  (set `self.counter` (+ (`self.counter`) DeltaSeconds))
  (`|ExecutionSequence`
    (:`then_0`
      (`self.K2_AddActorWorldOffset` (* (`self.velocity`) _returnvalue) true))
    (:`then_1`
      (bind _outactors (`GameplayStatics.GetAllActorsOfClass` "/Game/BPs/BP_Earth.BP_Earth_C"))
      (for _array_element _outactors
        (bind _returnvalue_2 (- (`SceneComponent.K2_GetComponentLocation` (`self.K2_GetRootComponent` _array_element)) (`SceneComponent.K2_GetComponentLocation` (`self.Sphere`))))
        (bind _output_get (set `self.Force` (/ (* (`self.G`) (`/Game/BPs/BP_Earth.Mass` _array_element)) (`KismetMathLibrary.MultiplyMultiply_FloatFloat` (`KismetMathLibrary.VSize` _returnvalue_2) 2.0))))
        (set `self.acceleration` (* (`KismetMathLibrary.Normal` _returnvalue_2) _output_get)))
      (set `self.velocity` (+ (* (`self.acceleration`) _returnvalue) (`self.velocity`))))
    (:`then_2`
      (if (>= (`self.counter`) 0.1)
        (`KismetSystemLibrary.DrawDebugPoint` (`SceneComponent.K2_GetComponentLocation` (`self.Sphere`)) 3.0 (struct :`R` 1.0 :`G` 1.0 :`B` 1.0 :`A` 1.0) 100.0)
        (set `self.counter` 0.0)))))

(event `self.Sphere.OnComponentBeginOverlap`
  (params (OverlappedComponent :type "PrimitiveComponent Object Reference") (OtherActor :type "Actor Object Reference") (OtherComp :type "PrimitiveComponent Object Reference") (OtherBodyIndex :type Integer) (bFromSweep :type Boolean) (SweepResult :type "HitResult Structure (by ref)"))
  (bind (_bblockinghit _binitialoverlap _time _location _impactpoint _normal) (`GameplayStatics.BreakHitResult` SweepResult))
  (cast `/Game/BPs/BP_Earth` OtherActor)
  (bind _returnvalue (`GameplayStatics.SpawnEmitterAtLocation` "/Game/StarterContent/Particles/P_Explosion.P_Explosion" _location (`KismetMathLibrary.Conv_VectorToRotator` _normal)))
  (`SceneComponent.SetRelativeScale3D` _returnvalue (50.0 50.0 50.0))
  (`self.K2_DestroyActor`))

(event `self.Sphere.OnComponentHit`
  (params (HitComponent :type "PrimitiveComponent Object Reference") (OtherActor :type "Actor Object Reference") (OtherComp :type "PrimitiveComponent Object Reference") (NormalImpulse :type "Vector Structure") (Hit :type "HitResult Structure (by ref)"))
  (bind _peoplekilled (`/Game/UI/HUD_WidgetBlueprint.PeopleKilled` (`/Game/BPs/BP_AsteroidSimulatorGM.HUDWidget` (`self.GM`))))
  (switch `EPhysicalSurface` (`PhysicalMaterial.SurfaceType` (`.PhysMat` (`GameplayStatics.BreakHitResult` Hit)))
    (:`SurfaceType_Default`
      (for _ (range 11)
        (`KismetSystemLibrary.PrintString` "Default")))
    (:`SurfaceType1`
      (for _ (range 11)
        (`KismetSystemLibrary.PrintString` "Europe")))
    (:`SurfaceType2`
      (set `self.Damage_Area` (* (`self.radius`) 4.0))
      (bind _output_get (set `self.Kills` (`KismetMathLibrary.FTrunc` (* (/ 1200000000.0 30370000.0) (`self.Damage_Area`)))))
      (`Widget.SetVisibility` _peoplekilled "Visible")
      (`TextBlock.SetText` _peoplekilled (`KismetTextLibrary.Conv_StringToText` (`KismetStringLibrary.Concat_StrStr` "People Killed: " (`KismetStringLibrary.Conv_IntToString` _output_get)))))))

(fn `SetRadius`
  (params (InRadius :type "Float (double-precision)"))
  (bind _staticmesh (`self.StaticMesh`))
  (set `self.radius` InRadius)
  (`SphereComponent.SetSphereRadius` (`self.Sphere`) (`self.radius`) true)
  (`SceneComponent.SetRelativeScale3D` _staticmesh (`KismetMathLibrary.Conv_DoubleToVector` (/ (* (`self.radius`) 8.0) (.y (`.BoxExtent` (`KismetSystemLibrary.GetComponentBounds` _staticmesh)))))))

(fn `UserConstructionScript`)