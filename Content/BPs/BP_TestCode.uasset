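; BP_TestCode is a scratch test Blueprint for checking large mass values and probing BP_Earth actors.
; On BeginPlay it sets Mass to a very large float, prints it, and stores all BP_Earth actors in the level.
; Unconnected experiments remain in the graph: an alternative Mass, a GravityRange debug sphere, and a printout of the distance to the first Earth.
; Tick and the construction script are empty.
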(event `self.ReceiveTick`
  (params (DeltaSeconds :type "Float (single-precision)")))

(event `self.ReceiveBeginPlay`
  (`|ExecutionSequence`
    (:`then_0`
      (bind _output_get (set `self.Mass` 5.97237e+19))
      (`KismetSystemLibrary.PrintString` (`KismetStringLibrary.Conv_DoubleToString` _output_get))
      (bind _outactors (`GameplayStatics.GetAllActorsOfClass` "/Game/BPs/BP_Earth.BP_Earth_C")))))

(fn `UserConstructionScript`)