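; BP_Earth is the Earth actor in the asteroid simulator, spinning about its vertical axis at one turn per simulated day.
; On BeginPlay it caches the simulator game mode and sets its rotation speed and mass, though mass is not used here.
; Each Tick applies a swept yaw rotation using delta time scaled by the game mode's TimeMultiplier.
; The construction script sizes both sphere components from Radius.
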(event `self.ReceiveBeginPlay`
  (bind _asbp_asteroid_simulator_gm (cast `/Game/BPs/BP_AsteroidSimulatorGM` (`GameplayStatics.GetGameMode`)))
  (set `self.AsteroidSimulatorGameMode` _asbp_asteroid_simulator_gm)
  (set `self.rotationSpeed` (/ 360.0 (* 60.0 60.0 24.0)))
  (set `self.Mass` 5.97219e+21))

(event `self.ReceiveTick`
  (params (DeltaSeconds :type "Float (single-precision)"))
  (`self.RotateAroundItsAxis` (* DeltaSeconds (`/Game/BPs/BP_AsteroidSimulatorGM.timeMultiplier` (`self.AsteroidSimulatorGameMode`)))))

(fn `RotateAroundItsAxis`
  (params (deltaTime :type "Float (double-precision)"))
  (`self.K2_AddActorWorldRotation` (`KismetMathLibrary.MakeRotator` 0.0 0.0 (* deltaTime (`self.rotationSpeed`))) true))

(fn `UserConstructionScript`
  (bind _returnvalue (* (`self.radius`) 2.0))
  (`SphereComponent.SetSphereRadius` (`self.Sphere1`) _returnvalue true)
  (`SceneComponent.SetRelativeScale3D` (`self.Sphere`) (`KismetMathLibrary.Conv_DoubleToVector` (* (/ _returnvalue 100.0) 2.0))))